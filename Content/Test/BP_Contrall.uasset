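; BP_Contrall is a player controller Blueprint that lets the player show and hide the main lobby widget.
; BeginPlay creates a BP_Lobby widget owned by the controller and stores it without displaying it.
; Each press of the ShowWedget input action toggles that same widget in the viewport and shows or hides the mouse cursor to match.
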(event `self.ReceiveBeginPlay`
  (bind _returnvalue (`|CreateWidget` "/Game/Test/BP_Lobby.BP_Lobby_C" self))
  (set `self.MainLobbyWidget` _returnvalue))

(event `InputAction|ShowWedget`
  (params (Key :type "Key Structure"))
  (bind _mainlobbywidget (`self.MainLobbyWidget`))
  (:`Pressed`
    (if (`Widget.IsInViewport` (`self.MainLobbyWidget`))
      (`Widget.RemoveFromParent` _mainlobbywidget)
      (set `self.bShowMouseCursor` false)
      (else
        (`UserWidget.AddToViewport` _mainlobbywidget 0)
        (set `self.bShowMouseCursor` true)))))

(fn `UserConstructionScript`)