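; BP_ShowChar is a test actor that spawns a row of BP_Char12 instances around its own location.
; On BeginPlay it loops PlayerCount times, spacing the spawns evenly along world X with an integer-halved index offset to roughly center the row.
; Spawns adjust for collisions but always succeed, and a debug greeting prints after the loop.
; Overlap, Tick and the construction script are empty.
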(event `self.ReceiveBeginPlay`
  (for _index (range (`self.PlayerCount`))
    (`|SpawnActorFromClass` "/Game/Test/BP_Char12.BP_Char12_C" (`KismetMathLibrary.Conv_VectorToTransform` (+ (`self.K2_GetActorLocation`) (`KismetMathLibrary.MakeVector` (`KismetMathLibrary.Conv_IntToDouble` (* (- _index (/ (`self.PlayerCount`) 2)) 100))))) "AdjustIfPossibleButAlwaysSpawn" "OverrideRootScale" null null))
  (`KismetSystemLibrary.PrintString` "Hello"))

(fn `UserConstructionScript`)